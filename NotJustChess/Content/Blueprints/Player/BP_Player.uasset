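; Player Blueprint for a turn-based, grid-based pawn game, handling camera rotation, view toggling and mouse interaction.
; Clicks line-trace toward the cursor, selecting pawns through BPI_Interact or, via state-dependent branches, validating moves with BP_GridManager and snapping pawns to cells.
; Tick drags a PhysicsHandle target under the cursor while Grabbing, but the grab setup is disconnected and GrabObject is empty.
; The enemy-turn handoff remains a placeholder.
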(event Custom|GrabObject)

(event Input|EnhancedActionEvents|EnhancedInputActionAI_Click
  (params (ActionValue :type Boolean) (ElapsedSeconds :type Float%20%28double-precision%29) (TriggeredSeconds :type Float%20%28double-precision%29) (InputAction :type Input%20Action%20Object%20Reference :default "/Game/Inputs/AI_Click.AI_Click"))
  ;[0.15 0.15 0.15 0.5] Tire un ray cast quand on click gauche
  (:Started
    (switch Utilities|FlowControl|Switch|SwitchonE_PlayerStates (Variables|Default|GetCurrent%20State)
      (:NewEnumerator0
        (bind _returnvalue (Actor|GetActorOfClass "/Game/Blueprints/Grid/BP_GridManager.BP_GridManager_C"))
        (Utilities|Array|AddUnique (Variables|Default|GetActors%20to%20Ignore) _returnvalue))
      (:NewEnumerator1
        (Utilities|Array|Clear (Variables|Default|GetActors%20to%20Ignore))))
    (bind (_outhit _returnvalue_2) (Collision|LineTraceByChannel "0, 0, 0" (.location (.HitResult (Game|Player|GetHitResultUnderCursorbyChannel (Game|GetPlayerController 0) "TraceTypeQuery2" true))) "TraceTypeQuery4" false (Variables|Default|GetActors%20to%20Ignore) "ForDuration" true "(R=1.000000,G=0.000000,B=0.000000,A=1.000000)" "(R=0.000000,G=1.000000,B=0.000000,A=1.000000)" 2.0))
    (switch Utilities|FlowControl|Switch|SwitchonE_PlayerStates (Variables|Default|GetCurrent%20State)
      (:NewEnumerator0
        (if _returnvalue_2
          (bind _asbpi_interact (Utilities|Casting|CastToBPI_Interact (.HitActor (Collision|BreakHitResult _outhit)))
            (:then
              (Default|Interact _asbpi_interact true)
              (Utilities|IsValid (Variables|Default|GetPawn%20Actor)
                (:Is%20Valid
                  (if (!= (Variables|Default|GetPawn%20Actor) (.HitActor (Collision|BreakHitResult _outhit)))
                    (bind _asbpi_interact_2 (Utilities|Casting|CastToBPI_Interact (Variables|Default|GetPawn%20Actor)))
                    (Default|Interact _asbpi_interact_2 false)
                    (Variables|Default|SetPawn%20Actor (.HitActor (Collision|BreakHitResult _outhit)))))
                (:Is%20Not%20Valid
                  (Variables|Default|SetPawn%20Actor (.HitActor (Collision|BreakHitResult _outhit))))))
            (:CastFailed
              (Development|PrintString (Utilities|GetDisplayName (.HitActor (Collision|BreakHitResult _outhit))))))
          (else
            (bind _asbp_grid_manager (Utilities|Casting|CastToBP_GridManager (.HitActor (Collision|BreakHitResult _outhit)) :!label _label))
            (bind _returnvalue_3 (Class|GridManager|MoveValidation _asbp_grid_manager))
            (if _returnvalue_3
              (Actor|Tick|SetActorTickEnabled false)
              ;;[0.15 0.15 1 0.5] A changer pour enemy turn
              (Variables|Default|SetCurrent%20State "NewEnumerator0")
              (Physics|Components|PhysicsHandle|ReleaseComponent (Variables|Default|GetPhysicsHandle))
              (Variables|Default|SetYPos (+ (Math|Conversions|ToFloat(Integer) (* (Math|Integer|%(Integer) (Variables|/Script/TRPG_Game.GridManager|GetCurrentIndex _asbp_grid_manager) (Variables|/Script/TRPG_Game.GridManager|GetY _asbp_grid_manager)) 100)) (.y (Transformation|GetActorLocation _asbp_grid_manager))))
              (Variables|Default|SetXPos (+ (Math|Conversions|ToFloat(Integer) (* (/ (Variables|/Script/TRPG_Game.GridManager|GetCurrentIndex _asbp_grid_manager) (Variables|/Script/TRPG_Game.GridManager|GetY _asbp_grid_manager)) 100)) (.x (Transformation|GetActorLocation _asbp_grid_manager))))
              (Transformation|SetActorLocation (Variables|Default|GetPawn%20Actor) (Math|Vector|MakeVector (Variables|Default|GetXPos) (Variables|Default|GetYPos) 1.0) false false)
              (Default|CallPlacePawn)
              (Variables|/Script/TRPG_Game.GridManager|SetCurrentAction _asbp_grid_manager 0)
              (Utilities|FlowControl|Delay 1.5)
              (Physics|SetSimulatePhysics (Actor|GetComponentbyClass (Variables|Default|GetPawn%20Actor) "/Script/Engine.MeshComponent") false)
              (Transformation|SetActorLocationAndRotation (Variables|Default|GetPawn%20Actor) (Math|Vector|MakeVector (Variables|Default|GetXPos) (Variables|Default|GetYPos) 1.0))
              (Variables|Default|SetPawn%20Actor 0)))))
      (:NewEnumerator1
        (goto _label)))))

(event Input|EnhancedActionEvents|EnhancedInputActionAI_Move
  (params (ActionValue :type Float%20%28double-precision%29) (ElapsedSeconds :type Float%20%28double-precision%29) (TriggeredSeconds :type Float%20%28double-precision%29) (InputAction :type Input%20Action%20Object%20Reference :default "/Game/Inputs/AI_Move.AI_Move"))
  ;[0.15 0.15 0.15 0.5] Gere les mouvement et la camera
  (Transformation|AddLocalRotation (Variables|Default|GetScene) (Math|Rotator|MakeRotator 0.0 0.0 (/ ActionValue (Variables|Default|GetRotation%20Force))) false false))

(event Input|EnhancedActionEvents|EnhancedInputActionAI_Camera
  (params (ActionValue :type Boolean) (ElapsedSeconds :type Float%20%28double-precision%29) (TriggeredSeconds :type Float%20%28double-precision%29) (InputAction :type Input%20Action%20Object%20Reference :default "/Game/Inputs/AI_Camera.AI_Camera"))
  (:Started
    (Utilities|FlowControl|FlipFlop
      (:A
        (Game|Player|SetViewTargetwithBlend (Game|GetPlayerController 0) (Variables|Default|GetCamera%20Level) 0.0 "VTBlend_Linear" 0.0 false))
      (:B
        (Game|Player|SetViewTargetwithBlend (Game|GetPlayerController 0) self 0.0 "VTBlend_Linear" 0.0 false)))))

(event EventBeginPlay
  (bind _returnvalue (Game|GetPlayerController 0))
  ;[0.15 0.15 0.15 0.5] Set les inputs et le cursor
  (Actor|Tick|SetActorTickEnabled false)
  (Input|AddMappingContext (PlayerController|LocalPlayerSubsystems|GetEnhancedInputLocalPlayerSubsystem _returnvalue) "/Game/Inputs/IMC.IMC" 0 "(bIgnoreAllPressedKeysUntilRelease=True,bForceImmediately=False,bNotifyUserSettings=False)")
  (Variables|/Script/Engine.PlayerController|SetbShowMouseCursor _returnvalue true)
  (bind _returnvalue_2 (Actor|GetActorOfClass "/Script/Engine.TargetPoint"))
  (Transformation|SetWorldLocation (Variables|Default|GetScene) (Transformation|GetWorldLocation (Variables|/Script/Engine.Actor|GetRootComponent _returnvalue_2)) false true)
  (bind _returnvalue_3 (Actor|GetActorOfClass "/Script/Engine.CameraActor"))
  (Variables|Default|SetCamera%20Level _returnvalue_3))

(event EventTick
  (params (DeltaSeconds :type Float%20%28single-precision%29))
  (bind _returnvalue (Game|GetPlayerController 0))
  (bind _hitresult (Game|Player|GetHitResultUnderCursorbyChannel _returnvalue "TraceTypeQuery4" true))
  (bind (_x _y) (Math|Vector|BreakVector (.location _hitresult)))
  ;[0.15 0.15 0.15 0.5] Fait bouger l'object avec la sourit
  (switch Utilities|FlowControl|Switch|SwitchonE_PlayerStates (Variables|Default|GetCurrent%20State)
    (:NewEnumerator1
      (Class|PhysicsHandleComponent|SetTargetLocationandRotation (Variables|Default|GetPhysicsHandle) (Math|Vector|MakeVector _x _y 2e+02) "0, 0, 0"))))

(fn ConstructionScript)