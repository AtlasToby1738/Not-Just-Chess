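; Grid manager for a turn-based pawn tactics game, handling turn handover, game end, pawn level-ups and visual feedback.
; Enemy turn end waits, checks for game over, then restores the player's state and action HUD, or the end event shows a result widget.
; Level-ups raise attack or health up to level two.
; Other events update HUD, promotion and downed-countdown widgets, play move sounds, and animate pawns to grid indices via a timeline.
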(event EventBeginPlay
  ;[0.15 0.15 0.15 0.5] Set player and hud ref
  (bind _asbp_players (Utilities|Casting|CastToBP_Players (Game|Player|GetPlayerPawn 0)))
  (Variables|Default|SetAs%20BP%20Players _asbp_players)
  (bind _asbp_hud (Utilities|Casting|CastToBP_HUD (HUD|GetHUD (Game|GetPlayerController 0))))
  (Variables|Default|SetAs%20BP%20HUD _asbp_hud))

(event EventCountEnemyPA
  (params (_pa :type Integer))
  (bind _as_bp_hud (Variables|Default|GetAs%20BP%20HUD))
  (bind _wbp_hud (Variables|/Game/Blueprints/BP_HUD.BP_HUD_C|GetWBP_HUD _as_bp_hud))
  ;[0.15 0.15 0.15 0.5] Update some visual
  ;;[0.15 0.15 0.15 0.5] PA visual for the enemy turn
  (Variables|/Game/Blueprints/Widgets/WBP_HUD.WBP_HUD_C|SetEnemyPA _wbp_hud _pa)
  (Default|SetPA _wbp_hud))

(event EventPlayMouveSound
  ;[0.15 0.15 0.15 0.5] Spawn sound on move
  (switch Utilities|FlowControl|Switch|SwitchonEPlayersStates (Variables|/Script/TRPG_Game.Players|GetCurrentState (Variables|Default|GetAs%20BP%20Players))
    (:PlayerTurn
      (Audio|SpawnSound2D "/Game/Sounds/2D/Move/SC_Move.SC_Move" 1.0 1.0 0.0 0 :!label _label))
    (:Grabbing
      (goto _label))
    (:Attacking
      (goto _label))
    (:EnemyTurn
      (Utilities|FlowControl|Delay 1.9)
      (Audio|SpawnSound2D "/Game/Sounds/2D/Move/SC_Move.SC_Move" 1.0 1.0 0.0 0))))

(event EventEndEnemyTurn
  ;[0.15 0.15 0.15 0.5] End the enemy turn and give it back to the player
  (Utilities|FlowControl|Delay 2.0)
  (bind _returnvalue (Class|GridManager|CheckforEnd))
  (if (not _returnvalue)
    (Default|CallEndOpponantTurn)
    (Variables|/Script/TRPG_Game.Players|SetCurrentState (Variables|Default|GetAs%20BP%20Players) "PlayerTurn")
    (Default|SetPA (Variables|/Game/Blueprints/BP_HUD.BP_HUD_C|GetWBP_HUD (Variables|Default|GetAs%20BP%20HUD)))
    (Variables|Default|SetCurrentAction 0)
    (Variables|Default|SetBonusActionsRemaining 0)))

(event EventMovePawnVisually
  (params (Pawn :type Pawns%20Object%20Reference) (Index :type Integer))
  (bind _returnvalue (Transformation|GetActorLocation))
  (bind _y (Variables|Default|GetY))
  ;[0.15 0.15 0.15 0.5] Update some visual
  ;;[0.15 0.15 0.15 0.5] Move the pawn for the enemy turn
  (Variables|Default|SetStart (Transformation|GetActorLocation Pawn))
  (Variables|Default|SetYPos (+ (Math|Conversions|ToFloat(Integer) (* (Math|Integer|%(Integer) Index _y) 100)) (.y _returnvalue)))
  (Variables|Default|SetXPos (+ (Math|Conversions|ToFloat(Integer) (* (/ Index _y) 100)) (.x _returnvalue)))
  (bind (_direction _alpha_x_y _alpha_z) (Timeline|Movement PlayFromStart)
    (:Update
      (Transformation|SetActorLocation Pawn (Math|Vector|MakeVector (Math|Float|Lerp (.x (Variables|Default|GetStart)) (Variables|Default|GetXPos) _alpha_x_y) (Math|Float|Lerp (.y (Variables|Default|GetStart)) (Variables|Default|GetYPos) _alpha_x_y) (Math|Float|Lerp 0.0 1e+02 _alpha_z)) false false))))

(event EventEndtheGame
  (params (Result :type EGameResult%20Enum :default "PlayerWin") (Reason :type EEndGameReason%20Enum :default "KingDefeated"))
  ;[0.15 0.15 0.15 0.5] End the game with the result the check found
  (Widget|RemovefromParent (Variables|/Game/Blueprints/BP_HUD.BP_HUD_C|GetWBP_HUD (Variables|Default|GetAs%20BP%20HUD)))
  (bind _returnvalue (UserInterface|CreateWidget "/Game/Blueprints/Widgets/WBP_End.WBP_End_C" 0 Result (Variables|Default|GetLevel) Reason))
  (UserInterface|Viewport|AddtoViewport _returnvalue 0)
  (Input|SetInputModeUIOnly (Game|GetPlayerController 0) 0 "DoNotLock" false))

(event EventOnBonusTurnGranted
  (params (_amount :type Integer))
  ;[0.15 0.15 0.15 0.5] Update some visual
  ;;[0.15 0.15 0.15 0.5] Bonus Turn Visual
  (Default|SetAdditionalTurn (Variables|Default|GetAs%20BP%20HUD) _amount))

(event EventOnDownedPawnCountdownUpdated
  (params (Pawn :type Pawns%20Object%20Reference) (TurnsRemaining :type Integer))
  ;[0.15 0.15 0.15 0.5] Update some visual
  ;;[0.15 0.15 0.15 0.5] Update the little time on top of the pawn when they are down
  (bind _asbp_pawns (Utilities|Casting|CastToBP_Pawns Pawn))
  (Default|UpdateDeathTimer _asbp_pawns TurnsRemaining))

(event EventOnPawnReadytoPromote
  (params (_awn :type Pawns%20Object%20Reference))
  ;[0.15 0.15 0.15 0.5] Update some visual
  ;;[0.15 0.15 0.15 0.5] Spawn the promotion widget on top of the pawn
  (bind _asbp_pawns (Utilities|Casting|CastToBP_Pawns _awn))
  (Default|SetPromotionWidget _asbp_pawns true))

(event EventLevelUpPawn
  (params (_pawn :type Pawns%20Object%20Reference) (_level :type Integer))
  (bind _returnvalue (Math|Integer|Clamp(Integer) _level 0 2))
  ;[0.15 0.15 0.15 0.5] Level Up Pawn
  (if (!= (.level (.pawnstats (Variables|/Script/TRPG_Game.Pawns|GetPawnStruct _pawn))) 2)
    (if (and (== (.level (.pawnstats (Variables|/Script/TRPG_Game.Pawns|GetPawnStruct _pawn))) 0) (== _returnvalue 1))
      (Variables|/Script/TRPG_Game.Pawns|SetPawnStruct _pawn (Utilities|Struct|MakePawnsStruct (.pawntype (Variables|/Script/TRPG_Game.Pawns|GetPawnStruct _pawn)) (.pawnteam (Variables|/Script/TRPG_Game.Pawns|GetPawnStruct _pawn)) (.pawnname (Variables|/Script/TRPG_Game.Pawns|GetPawnStruct _pawn)) (Utilities|Struct|MakePawnStats (+ (.attack (.pawnstats (Variables|/Script/TRPG_Game.Pawns|GetPawnStruct _pawn))) 2) (.health (.pawnstats (Variables|/Script/TRPG_Game.Pawns|GetPawnStruct _pawn))) (.maxhealth (.pawnstats (Variables|/Script/TRPG_Game.Pawns|GetPawnStruct _pawn))) 1 (.size (.pawnstats (Variables|/Script/TRPG_Game.Pawns|GetPawnStruct _pawn))))))
      (elif (and (== (.level (.pawnstats (Variables|/Script/TRPG_Game.Pawns|GetPawnStruct _pawn))) 1) (== _returnvalue 1))
        (Variables|/Script/TRPG_Game.Pawns|SetPawnStruct _pawn (Utilities|Struct|MakePawnsStruct (.pawntype (Variables|/Script/TRPG_Game.Pawns|GetPawnStruct _pawn)) (.pawnteam (Variables|/Script/TRPG_Game.Pawns|GetPawnStruct _pawn)) (.pawnname (Variables|/Script/TRPG_Game.Pawns|GetPawnStruct _pawn)) (Utilities|Struct|MakePawnStats (.attack (.pawnstats (Variables|/Script/TRPG_Game.Pawns|GetPawnStruct _pawn))) (+ (.health (.pawnstats (Variables|/Script/TRPG_Game.Pawns|GetPawnStruct _pawn))) 2) (+ (.maxhealth (.pawnstats (Variables|/Script/TRPG_Game.Pawns|GetPawnStruct _pawn))) 2) 2 (.size (.pawnstats (Variables|/Script/TRPG_Game.Pawns|GetPawnStruct _pawn))))))
        (else
          (Variables|/Script/TRPG_Game.Pawns|SetPawnStruct _pawn (Utilities|Struct|MakePawnsStruct (.pawntype (Variables|/Script/TRPG_Game.Pawns|GetPawnStruct _pawn)) (.pawnteam (Variables|/Script/TRPG_Game.Pawns|GetPawnStruct _pawn)) (.pawnname (Variables|/Script/TRPG_Game.Pawns|GetPawnStruct _pawn)) (Utilities|Struct|MakePawnStats (+ (.attack (.pawnstats (Variables|/Script/TRPG_Game.Pawns|GetPawnStruct _pawn))) 2) (+ (.health (.pawnstats (Variables|/Script/TRPG_Game.Pawns|GetPawnStruct _pawn))) 2) (+ (.maxhealth (.pawnstats (Variables|/Script/TRPG_Game.Pawns|GetPawnStruct _pawn))) 2) 2 (.size (.pawnstats (Variables|/Script/TRPG_Game.Pawns|GetPawnStruct _pawn)))))))))
    (bind _asbp_pawns (Utilities|Casting|CastToBP_Pawns _pawn))
    (Default|UpdateLevelHUD _asbp_pawns)
    (Class|Pawns|UpdateLifeHUD _asbp_pawns)))

(fn ConstructionScript)