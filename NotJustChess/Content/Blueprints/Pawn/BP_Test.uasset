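; BP_Test is a chess-style piece on a BP_GridManager grid, with mesh and material chosen by type and team in the construction script.
; Interact toggles the piece's widget and the Selected state of its tile, found by a downward line trace that also sets the grid's start index.
; RangeCheck only handles Pawn, one grid row forward.
; Widget binding, GridRef assignment and tile-occupancy logic are disconnected and never run.
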(event Custom|Closing
  (if (Rendering|IsVisible (Variables|Default|GetWidget))
    (Rendering|SetVisibility (Variables|Default|GetWidget) false false)))

(event Custom|WhenPlacedGetCalled)

(event EventBeginPlay
  (bind _returnvalue (Actor|GetActorOfClass "/Game/Blueprints/Player/BP_Players.BP_Players_C"))
  (Variables|Default|SetPlayerRef _returnvalue))

(event EventInteract
  (params (IsActif%20? :type Boolean))
  (if (and IsActif%20? (not (Rendering|IsVisible (Variables|Default|GetWidget))))
    (Rendering|SetVisibility (Variables|Default|GetWidget) true false)
    (bind (_asbp_grid_manager _hititem) (CallFunction|GetCurrentTyleIndex))
    (bind _output_get (Variables|Default|SetCurrent%20Index _hititem))
    (Class|GridManager|AddStatetoTile _asbp_grid_manager "Selected" _output_get)
    (else
      (Rendering|SetVisibility (Variables|Default|GetWidget) false false)
      (Class|GridManager|RemoveStatetoTile (Variables|Default|GetGridRef) "Selected" (Variables|Default|GetCurrent%20Index))
      (Variables|Default|SetCurrent%20Index -1))))

(fn ConstructionScript
  (Components|StaticMesh|SetStaticMesh (Variables|Default|GetStaticMesh) (Utilities|Select :Index (.type (Variables|Default|GetPawn%20Information)) :NewEnumerator0 "/Game/Assets/Pawn.Pawn" :NewEnumerator1 "/Game/Assets/King.King" :NewEnumerator2 "/Game/Assets/Cube1X1.Cube1X1" :NewEnumerator3 "/Game/Assets/Tower.Tower" :NewEnumerator4 "/Game/Assets/Bishop.Bishop" :NewEnumerator5 "/Game/Assets/Queen.Queen"))
  (Rendering|Material|SetMaterial (Variables|Default|GetStaticMesh) 0 (Utilities|Select :Index (.team (Variables|Default|GetPawn%20Information)) :NewEnumerator0 "/Game/Assets/Cercle.Cercle" :NewEnumerator1 "/Game/Assets/Plane.Plane")))

(fn GetCurrentTyleIndex
  (bind _scene (Variables|Default|GetScene))
  (bind _returnvalue (Transformation|GetWorldLocation _scene))
  (bind (_outhit _returnvalue_2) (Collision|LineTraceByChannel _returnvalue (- _returnvalue "0.000000,0.000000,500.000000") "TraceTypeQuery3" false 0 "None"))
  (if _returnvalue_2
    (bind _asbp_grid_manager (Utilities|Casting|CastToBP_GridManager (.HitActor (Collision|BreakHitResult _outhit))))
    (Class|GridManager|SetStartIndex _asbp_grid_manager (.HitItem (Collision|BreakHitResult _outhit)))
    (return _asbp_grid_manager (.HitItem (Collision|BreakHitResult _outhit)))))

(fn RangeCheck
  (params (New%20Case%20Index :type Integer) (Grid%20Size :type Integer))
  (LocalVariables|SetCase%20Index New%20Case%20Index)
  (LocalVariables|SetSize Grid%20Size)
  (switch Utilities|FlowControl|Switch|SwitchonE_PawnType (.type (Variables|Default|GetPawn%20Information))
    (:NewEnumerator0
      (return (== (+ (Variables|Default|GetCurrent%20Index) (LocalVariables|GetSize)) (LocalVariables|GetCase%20Index))))))