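; Chess piece pawn for a grid battle game, with type, team, health and level, ending the game when a King reaches zero health.
; Piece type drives mesh and stats, team sets color, and a dissolve material tracks the death timer.
; Downward traces register it with BP_GridManager and find its tile for selection.
; Widget components show stats, abilities, death countdown and promotion, linked to the pawn, player or grid.
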(event Custom|Closing
  (if (Rendering|IsVisible (Variables|Default|GetAbility))
    (Rendering|SetVisibility (Variables|Default|GetAbility) false false)))

(event Custom|UpdateDeathTimer
  (params (Turns%20Left :type Integer))
  (bind _death (Variables|Default|GetDeath))
  (Rendering|Material|SetScalarParameterValueonMaterials (Variables|Default|GetStaticMesh) "Slider" (- (/ (Math|Conversions|ToFloat(Integer) Turns%20Left) 3.0) 0.1))
  (Rendering|SetVisibility _death true false)
  (bind _aswbp_death_timer (Utilities|Casting|CastToWBP_DeathTimer (UserInterface|GetWidget _death)))
  (Default|SetDeathTimer _aswbp_death_timer Turns%20Left))

(event Custom|Set%20PromotionWidget
  (params (State :type Boolean))
  (bind _promotion (Variables|Default|GetPromotion))
  (bind _aswbp_promotion (Utilities|Casting|CastToWBP_Promotion (UserInterface|GetWidget _promotion)))
  (Variables|/Game/Blueprints/Widgets/WBP_Promotion.WBP_Promotion_C|SetBP_Grid _aswbp_promotion (Variables|Default|GetGridRef))
  (Variables|/Game/Blueprints/Widgets/WBP_Promotion.WBP_Promotion_C|SetPawn _aswbp_promotion self)
  (Variables|/Game/Blueprints/Widgets/WBP_Promotion.WBP_Promotion_C|SetPlayer _aswbp_promotion (Variables|Default|GetPlayerRef))
  (Rendering|SetVisibility _promotion State false))

(event Custom|UpdateLevelHUD
  (Default|UpdateLvl (Variables|Default|GetAs%20WBP%20Stats) false))

(event EventBeginPlay
  (bind _scene (Variables|Default|GetScene))
  (bind _returnvalue (Transformation|GetWorldLocation _scene))
  (bind _aswbp_stats (Utilities|Casting|CastToWBP_Stats (UserInterface|GetWidget (Variables|Default|GetStats))))
  (bind _output_get (Variables|Default|SetAs%20WBP%20Stats _aswbp_stats))
  (Variables|/Game/Blueprints/Widgets/WBP_Stats.WBP_Stats_C|SetParent _output_get self)
  (bind _returnvalue_2 (Actor|GetActorOfClass "/Game/Blueprints/Player/BP_Players.BP_Players_C"))
  (Variables|Default|SetPlayerRef _returnvalue_2)
  (bind _aswbp_pawn (Utilities|Casting|CastToWBP_Pawn (UserInterface|GetWidget (Variables|Default|GetAbility))))
  (EventDispatchers|BindEventtoClosing _aswbp_pawn (delegate Custom|Closing))
  (Variables|/Game/Blueprints/Widgets/WBP_Pawn.WBP_Pawn_C|SetParent _aswbp_pawn self)
  (Variables|/Game/Blueprints/Widgets/WBP_Pawn.WBP_Pawn_C|SetPlayer _aswbp_pawn (Variables|Default|GetPlayerRef))
  (bind (_outhit _returnvalue_3) (Collision|LineTraceByChannel _returnvalue (- _returnvalue "0.000000,0.000000,500.000000") "TraceTypeQuery3" false 0 "None"))
  (if _returnvalue_3
    (bind _asbp_grid_manager (Utilities|Casting|CastToBP_GridManager (.HitActor (Collision|BreakHitResult _outhit))))
    (bind _output_get_2 (Variables|Default|SetGridRef _asbp_grid_manager))
    (Class|GridManager|SpawnPawns _output_get_2 (.HitItem (Collision|BreakHitResult _outhit)) self)
    (Variables|Default|SetIndex (.HitItem (Collision|BreakHitResult _outhit)))))

(event EventUpdateLifeHUD
  (bind _pawnstruct (Variables|Default|GetPawnStruct))
  (Audio|SpawnSound2D "/Game/Sounds/2D/Hits/SC_Hit.SC_Hit" 1.0 1.0 0.0 0)
  (Default|SetLifeAmount (Variables|Default|GetAs%20WBP%20Stats) (Math|Conversions|ToFloat(Integer) (.health (.pawnstats _pawnstruct))))
  (if (and (<= (.health (.pawnstats _pawnstruct)) 0) (Utilities|Enum|Equal(Enum) (.pawntype _pawnstruct) "King"))
    (Utilities|FlowControl|Delay 2.0)
    (Class|GridManager|EndtheGame (Variables|Default|GetGridRef) (Utilities|Select :Index (.pawnteam _pawnstruct) :None "PlayerWin" :Ally "OpponentWin" :Opponent "PlayerWin") "KingDefeated")))

(event EventUpdateVisualonPromotionIA
  (Utilities|FlowControl|Delay 2.0)
  (CallFunction|SetthePawnbyType false)
  (Default|InitialezStat (Variables|Default|GetAs%20WBP%20Stats)))

(event EventInteract
  (params (IsActif%20? :type Boolean))
  (if (and IsActif%20? (not (Rendering|IsVisible (Variables|Default|GetAbility))))
    (Rendering|SetVisibility (Variables|Default|GetAbility) true false)
    (bind (_asbp_grid_manager _hititem) (CallFunction|GetCurrentTyleIndex))
    (bind _output_get (Variables|Default|SetIndex _hititem))
    (Class|GridManager|AddStatetoTile _asbp_grid_manager "Selected" _output_get)
    (else
      (Rendering|SetVisibility (Variables|Default|GetAbility) false false)
      (Class|GridManager|RemoveStatetoTile (Variables|Default|GetGridRef) "Selected" (Variables|Default|GetIndex))))
  (Variables|Default|SetLast%20Location (Transformation|GetActorLocation)))

(fn ConstructionScript
  (Rendering|Material|SetMaterial (Variables|Default|GetStaticMesh) 0 "/Game/Materials/M_GradualDisappearance.M_GradualDisappearance")
  (CallFunction|SetthePawnbyType false)
  (Rendering|Material|SetColorParameterValueonMaterials (Variables|Default|GetStaticMesh) "Color" (Utilities|Select :Index (.pawnteam (Variables|Default|GetPawnStruct)) :None "" :Ally "(R=1.000000,G=1.000000,B=1.000000,A=1.000000)" :Opponent "")))

(fn GetCurrentTyleIndex
  (bind _staticmesh (Variables|Default|GetStaticMesh))
  (bind _returnvalue (Transformation|GetWorldLocation _staticmesh))
  (bind (_outhit _returnvalue_2) (Collision|LineTraceByChannel _returnvalue (- _returnvalue "0.000000,0.000000,500.000000") "TraceTypeQuery3" false 0 "None"))
  (if _returnvalue_2
    (bind _asbp_grid_manager (Utilities|Casting|CastToBP_GridManager (.HitActor (Collision|BreakHitResult _outhit))))
    (Class|GridManager|SetStartIndex _asbp_grid_manager (.HitItem (Collision|BreakHitResult _outhit)))
    (return _asbp_grid_manager (.HitItem (Collision|BreakHitResult _outhit)))))

(fn SetthePawnbyType
  (params (Promotion? :type Boolean))
  (Variables|Default|SetPawnStruct (Utilities|Struct|MakePawnsStruct (.pawntype (Variables|Default|GetPawnStruct)) (.pawnteam (Variables|Default|GetPawnStruct)) (Utilities|Name|EnumtoName (.pawntype (Variables|Default|GetPawnStruct))) (Utilities|Struct|MakePawnStats (Utilities|Select :Index (.pawntype (Variables|Default|GetPawnStruct)) :None 0 :Pawn 1 :King 2 :Knight 2 :Tower 1 :Bishop 1 :Queen 2) (select Promotion? (Utilities|Select :Index (.pawntype (Variables|Default|GetPawnStruct)) :None 0 :Pawn 2 :King 4 :Knight 4 :Tower 6 :Bishop 4 :Queen 5) (.health (.pawnstats (Variables|Default|GetPawnStruct)))) (Utilities|Select :Index (.pawntype (Variables|Default|GetPawnStruct)) :None 0 :Pawn 2 :King 4 :Knight 4 :Tower 6 :Bishop 4 :Queen 5) (.level (.pawnstats (Variables|Default|GetPawnStruct))) (Utilities|Select :Index (.pawntype (Variables|Default|GetPawnStruct)) :None 0 :Pawn 93 :King 150 :Knight 100 :Tower 130 :Bishop 120 :Queen 130))))
  (Components|StaticMesh|SetStaticMesh (Variables|Default|GetStaticMesh) (Utilities|Select :Index (.pawntype (Variables|Default|GetPawnStruct)) :None "/Game/Assets/Cube1X1.Cube1X1" :Pawn "/Game/Assets/Pawn.Pawn" :King "/Game/Assets/King.King" :Knight "/Game/Assets/Knight.Knight" :Tower "/Game/Assets/Tower.Tower" :Bishop "/Game/Assets/Bishop.Bishop" :Queen "/Game/Assets/Queen.Queen"))
  (Rendering|Material|SetScalarParameterValueonMaterials (Variables|Default|GetStaticMesh) "Size" (Math|Conversions|ToFloat(Integer) (.size (.pawnstats (Variables|Default|GetPawnStruct)))))
  (Variables|Default|SetPawnStruct (Utilities|Struct|MakePawnsStruct (.pawntype (Variables|Default|GetPawnStruct)) (.pawnteam (Variables|Default|GetPawnStruct)) (Utilities|String|StringToName (Utilities|String|EnumtoString (.pawntype (Variables|Default|GetPawnStruct)))) (.pawnstats (Variables|Default|GetPawnStruct)))))